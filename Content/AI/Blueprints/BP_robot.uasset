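; BP_robot is an AI-controlled robot that fetches bananas and drops them near the player.
; Hitting an actor tagged true_banan disables its collision, attaches it to a mesh socket and clears the blackboard's banana key.
; Overlapping the BP_TPC character while carrying one detaches it, restoring collision after a short delay.
; The TPCtoBb interface event writes the player character into the blackboard.
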(event `self.ReceiveActorBeginOverlap`
  (params (OtherActor :type "Actor Object Reference")))

(event `self.CapsuleComponent.OnComponentHit`
  (params (HitComponent :type "PrimitiveComponent Object Reference") (OtherActor :type "Actor Object Reference") (OtherComp :type "PrimitiveComponent Object Reference") (NormalImpulse :type "Vector Structure") (Hit :type "HitResult Structure (by ref)"))
  ;[1 1 1] Robot picking up a banana on hit one
  (if (`self.ActorHasTag` OtherActor "true_banan")
    (set `self.banan` OtherActor)
    (`self.SetActorEnableCollision` (`self.banan`) false)
    (`KismetSystemLibrary.PrintString` "yes, sir")
    (`self.K2_AttachToComponent` (`self.banan`) (`self.Mesh`) "Socket_for_banan" "SnapToTarget" "SnapToTarget" "KeepWorld" true)
    (`BlackboardComponent.ClearValue` (`AIController.Blackboard` (`AIBlueprintHelperLibrary.GetAIController` self)) "banan")
    (set `self.has_banan` true)))

(event `self.CapsuleComponent.OnComponentBeginOverlap`
  (params (OverlappedComponent :type "PrimitiveComponent Object Reference") (OtherActor :type "Actor Object Reference") (OtherComp :type "PrimitiveComponent Object Reference") (OtherBodyIndex :type Integer) (bFromSweep :type Boolean) (SweepResult :type "HitResult Structure (by ref)"))
  ;[1 1 1] Robot leaving a banana near the player
  (cast `/Game/ThirdPerson/Blueprints/BP_TPC` OtherActor)
  (if (`self.has_banan`)
    (`/Game/ThirdPerson/Blueprints/BP_interface.Drop_banan`)))

(event `/Game/ThirdPerson/Blueprints/BP_interface.TPC_to_bb`
  ;[1 1 1] See BP_interface
  (`BlackboardComponent.SetValueAsObject` (`AIController.Blackboard` (`AIBlueprintHelperLibrary.GetAIController` self)) "TPC" (`GameplayStatics.GetPlayerCharacter` 0)))

(event `/Game/ThirdPerson/Blueprints/BP_interface.Drop_banan`
  (bind _banan (`self.banan`))
  ;[1 1 1] See BP_interface
  (`self.K2_DetachFromActor` _banan "KeepWorld" "KeepRelative" "KeepWorld")
  (set `self.has_banan` false)
  (`KismetSystemLibrary.Delay` 1.0)
  (`self.SetActorEnableCollision` _banan true))

(fn `UserConstructionScript`)